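; AI controller for bandit enemies that runs the BT_Bandits behavior tree when play begins.
; BeginPlay writes the player character and a one-time snapshot of its location to the blackboard, then caches the controlled pawn as BP_HeavyBandit.
; MoveAccordingly turns the heavy bandit's sprite to one of two opposite rotations by comparing the controller's X position with the player's, but nothing in this file calls it.
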(event `self.ReceiveBeginPlay`
  (bind _returnvalue (`GameplayStatics.GetPlayerCharacter` 0))
  (bind _returnvalue_2 (`AIBlueprintHelperLibrary.GetBlackboard` null))
  (`self.RunBehaviorTree` "/Game/Enemies/AI/BT_Bandits.BT_Bandits")
  (`BlackboardComponent.SetValueAsVector` _returnvalue_2 "PlayerLocation" (`self.K2_GetActorLocation` _returnvalue))
  (`BlackboardComponent.SetValueAsObject` _returnvalue_2 "Player" _returnvalue)
  (bind _asbp_heavy_bandit (cast `/Game/Enemies/Blueprints/BP_HeavyBandit` (`self.K2_GetPawn`)))
  (set `self.As BP Heavy Bandit` _asbp_heavy_bandit))

(event `self.ReceiveTick`
  (params (DeltaSeconds :type "Float (single-precision)")))

(fn `MoveAccordingly`
  (bind _returnvalue_x (`KismetMathLibrary.BreakVector` (`self.K2_GetActorLocation`)))
  (bind _returnvalue_x_2 (`KismetMathLibrary.BreakVector` (`self.K2_GetActorLocation` (`GameplayStatics.GetPlayerCharacter` 0))))
  (if (> _returnvalue_x _returnvalue_x_2)
    (bind _asbp_heavy_bandit (cast `/Game/Enemies/Blueprints/BP_HeavyBandit` (`self.K2_GetPawn`)))
    (`SceneComponent.K2_SetWorldRotation` :`self` (`PaperCharacter.Sprite` _asbp_heavy_bandit))
    (else
      (bind _asbp_heavy_bandit_2 (cast `/Game/Enemies/Blueprints/BP_HeavyBandit` (`self.K2_GetPawn`)))
      (`SceneComponent.K2_SetWorldRotation` (`PaperCharacter.Sprite` _asbp_heavy_bandit_2) (struct :`Yaw` 180.0) false false))))

(fn `UserConstructionScript`)