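; BP_Glena is a pawn blueprint that turns Glena to face left or right based on horizontal movement.
; Each Tick it checks the sign of X velocity and snaps the control rotation yaw forward or backward, using BisMovingRight to pick the facing when stationary.
; Tick also prints IsTakingDamage every frame as debug output.
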(event `self.ReceiveTick`
  (params (DeltaSeconds :type "Float (single-precision)"))
  (bind _returnvalue (`self.GetController`))
  (bind _returnvalue_2 (`self.GetController`))
  (`KismetSystemLibrary.PrintString` (`KismetStringLibrary.Conv_BoolToString` (`self.isTakingDamage`)))
  (`/Engine/EditorBlueprintResources/StandardMacros.CompareFloat` (.x (`MovementComponent.Velocity` (`self.GetMovementComponent`)))
    (:`>`
      (`/Engine/EditorBlueprintResources/StandardMacros.IsValid` _returnvalue_2 :!label _label
        (:`Is Valid`
          (`Controller.SetControlRotation` _returnvalue_2 (`KismetMathLibrary.MakeRotator` 0.0)))))
    (:`==`
      (if (`self.bisMovingRight`)
        (goto _label)
        (else
          (`/Engine/EditorBlueprintResources/StandardMacros.IsValid` _returnvalue :!label _label_2
            (:`Is Valid`
              (`Controller.SetControlRotation` _returnvalue (`KismetMathLibrary.MakeRotator` 0.0 0.0 180.0)))))))
    (:`<`
      (goto _label_2))))

(fn `UserConstructionScript`)